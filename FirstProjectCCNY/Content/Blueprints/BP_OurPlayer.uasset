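; BP_OurPlayer is the player pawn, handling movement, looking, jumping and coin pickups.
; BeginPlay adds the PlayerControls Enhanced Input mapping context, whose actions drive jump, controller yaw/pitch and movement relative to control yaw.
; Only sideways input is scaled by WalkSpeed.
; The custom PickUpCoin event increments and prints the Coin count, then prints "Hello" once the threshold is reached.
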(event `self.ReceiveBeginPlay`
  (bind _asplayer_controller (cast `PlayerController` (`self.GetController`)))
  (message `EnhancedInputSubsystemInterface.AddMappingContext` (pcsubsystem `EnhancedInputLocalPlayerSubsystem` _asplayer_controller) "/Game/PlayerControls.PlayerControls" 0 (struct)))

(event `EnhancedInput|/Game/Jump`
  (params (ActionValue :type Boolean) (ElapsedSeconds :type "Float (double-precision)") (TriggeredSeconds :type "Float (double-precision)") (InputAction :type "InputAction Object Reference" :default "/Game/Jump.Jump"))
  (:`Triggered`
    (`self.Jump`)))

(event `EnhancedInput|/Game/TurnHead`
  (params (ActionValue :type "Float (double-precision)") (ElapsedSeconds :type "Float (double-precision)") (TriggeredSeconds :type "Float (double-precision)") (InputAction :type "InputAction Object Reference" :default "/Game/TurnHead.TurnHead"))
  (:`Triggered`
    (`self.AddControllerYawInput` ActionValue)))

(event `PickUpCoin`
  ; made custom event that adds to our var coin
  (bind _output_get (set `self.Coin` (+ (`self.Coin`) 1)))
  (`KismetSystemLibrary.PrintString` (`KismetStringLibrary.Concat_StrStr` "Collected: " (`KismetStringLibrary.Conv_IntToString` _output_get)))
  ; checks if we collected enough coins
  (if (>= (`self.Coin`) 2)
    (`KismetSystemLibrary.PrintString` "Hello")))

(event `EnhancedInput|/Game/LookUp`
  (params (ActionValue :type "Float (double-precision)") (ElapsedSeconds :type "Float (double-precision)") (TriggeredSeconds :type "Float (double-precision)") (InputAction :type "InputAction Object Reference" :default "/Game/LookUp.LookUp"))
  (:`Triggered`
    (`self.AddControllerPitchInput` (* -1.0 ActionValue))))

(event `EnhancedInput|/Game/WalkForward`
  (params (ActionValue :type "Float (double-precision)") (ElapsedSeconds :type "Float (double-precision)") (TriggeredSeconds :type "Float (double-precision)") (InputAction :type "InputAction Object Reference" :default "/Game/WalkForward.WalkForward"))
  ; more complicated bc it has to take in account of the direction we are looking
  (:`Triggered`
    (`self.AddMovementInput` (`KismetMathLibrary.GetForwardVector` (`KismetMathLibrary.MakeRotator` 0.0 0.0 (.yaw (`self.GetControlRotation`)))) ActionValue)))

(event `EnhancedInput|/Game/WalkRight`
  (params (ActionValue :type "Float (double-precision)") (ElapsedSeconds :type "Float (double-precision)") (TriggeredSeconds :type "Float (double-precision)") (InputAction :type "InputAction Object Reference" :default "/Game/WalkRight.WalkRight"))
  (:`Triggered`
    (`self.AddMovementInput` (`KismetMathLibrary.GetRightVector` (`KismetMathLibrary.MakeRotator` 0.0 0.0 (.yaw (`self.GetControlRotation`)))) (* ActionValue (`self.walkSpeed`)))))

(fn `UserConstructionScript`)